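; Player pawn with tracked hands that can recognize hand signs from finger bone positions.
; BeginPlay caches bone names from the right hand's bone mappings, and a delayed Tick prints their component-space locations about once a second as debug output.
; ReadHandSign compares a given hand's bone locations to each AvailableSigns entry within ReadingAccuracy and returns the first full match.
; Nothing in this Blueprint calls ReadHandSign.
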(event `self.ReceiveBeginPlay`
  (bind _values (`BlueprintMapLibrary.Map_Values` (`OculusHandComponent.BoneNameMappings` (`self.HandR`))))
  (set `self.BoneNames` _values))

(event `self.ReceiveTick`
  (params (DeltaSeconds :type "Float (single-precision)"))
  (bind _handr (`self.HandR`))
  (`KismetSystemLibrary.Delay` 1.0)
  (for _index (range 25)
    (bind _output (`|GetArrayItem` (`self.BoneNames`) _index))
    (`PoseableMeshComponent.GetBoneLocationByName` _handr _output "ComponentSpace")
    (bind _returnvalue_location (`KismetMathLibrary.BreakTransform` (`SceneComponent.GetSocketTransform` _handr _output "RTS_Component")))
    (`KismetSystemLibrary.PrintString` (`KismetStringLibrary.Concat_StrStr` (`KismetStringLibrary.Conv_NameToString` _output) ": " (`KismetStringLibrary.Conv_VectorToString` _returnvalue_location)))))

(fn `ReadHandSign`
  (params (Hand :type "PoseableMeshComponent Object Reference"))
  (returns (ReturnedSign :type "/Game/Blueprints/Data/SignStruct Structure"))
  (locals (SignIndex :type Integer) (CorrectLocation :type Boolean))
  (for (_array_element _array_index) (`self.AvailableSigns`)
    ;[1 1 1] Comparing finger locations to existing ones
    (for (_array_element_2 _array_index_2) (`.BoneLoc_7_2B2D571A4859DB60C2BCA3B556599016` (break `/Game/Blueprints/Data/SignStruct` _array_element))
      (bind _returnvalue (`PoseableMeshComponent.GetBoneLocationByName` (`local.Hand`) (`|GetArrayItem` (`self.BoneNames`) _array_index_2) "ComponentSpace"))
      (bind _output_get (set `local.CorrectLocation` (== _array_element_2 _returnvalue :`ErrorTolerance` (`self.ReadingAccuracy`))))
      (if (not _output_get)
        (break)))
    (if (`local.CorrectLocation`)
      (set `local.SignIndex` _array_index)
      (break)))
  (if (`local.CorrectLocation`)
    (return (`|GetArrayItem` (`self.AvailableSigns`) (`local.SignIndex`)))
    (else
      (return))))

(fn `UserConstructionScript`)